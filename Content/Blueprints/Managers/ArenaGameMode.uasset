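; Server-side game mode for a multiplayer arena that handles player joining, game stop and game reset.
; BeginPlay caches spawn points, waiting and queue zones and the game and reset managers, then starts a looping timer.
; PostLogin queues controllers, which the timer processes by spawning and possessing a character in the QueueZone, refreshing colors and destroying Mur actors.
; ResetGame clears characters, frees waiting zones and re-queues controllers for respawn, while StopGame disables characters.
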(event Custom|OnPostLogin
  (bind _playerstryingtojoin (Variables|Default|GetPlayersTryingToJoin))
  (bind _queuezone (Variables|Default|GetQueueZone))
  (bind _spawnpoint (Variables|/Game/Blueprints/QueueZone.QueueZone_C|GetSpawnPoint _queuezone))
  (bind _returnvalue (Transformation|GetWorldTransform _spawnpoint))
  (Networking|SwitchHasAuthority
    (:Authority
      (if (!= (Utilities|Array|Length _playerstryingtojoin) 0)
        (bind _ascontroller (Utilities|Casting|CastToController (Utilities|Array|Get(acopy) _playerstryingtojoin)))
        (bind _output_get (Variables|Default|SetJoiningPlayer _ascontroller))
        (Utilities|Array|AddUnique (Variables|Default|GetPlayerControllerList) _output_get)
        (Utilities|FlowControl|Delay 0.1)
        (bind _returnvalue_2 (Game|SpawnActorfromClass "/Game/Blueprints/MyCharacter2.MyCharacter2_C" (Math|Transform|MakeTransform (.location _returnvalue) (.rotation _returnvalue) "1,1,1") "AdjustIfPossibleButAlwaysSpawn" 0 0))
        (Default|AddPlayer (Variables|Default|GetQueueZone) _returnvalue_2)
        (Pawn|Possess (Variables|Default|GetJoiningPlayer) _returnvalue_2)
        (bind _returnvalue_3 (Utilities|Array|AddUnique (Variables|Default|GetPlayerList) _returnvalue_2))
        (Variables|/Game/Blueprints/MyCharacter2.MyCharacter2_C|SetplayerIndex _returnvalue_2 _returnvalue_3)
        (Variables|/Game/Blueprints/Managers/Controller.Controller_C|SetControlledCharacter (Variables|Default|GetJoiningPlayer) _returnvalue_2)
        (Default|InitCam (Variables|Default|GetJoiningPlayer))
        (for _array_element (Variables|Default|GetPlayerList)
          (Default|RefreshColors _array_element))
        (bind _outactors (Actor|GetAllActorsOfClass "/Game/Blueprints/Mur.Mur_C"))
        (for _array_element_2 _outactors
          (Default|DestroyFast _array_element_2)
          (Utilities|Array|RemoveItem (Variables|Default|GetPlayersTryingToJoin) (Variables|Default|GetJoiningPlayer)))))))

(event Custom|ResetGame
  (bind _playercontrollerlist (Variables|Default|GetPlayerControllerList))
  (bind _playerlist (Variables|Default|GetPlayerList))
  (Default|DestroyCameraandPlayers (Variables|Default|GetResetManager))
  (for _array_element _playerlist
    (Actor|DestroyActor _array_element))
  (for _array_element_2 (Variables|Default|GetWaitingZonePoints)
    (Variables|/Game/Blueprints/WaitingZone.WaitingZone_C|SetFree _array_element_2 true))
  (Utilities|Array|Clear _playerlist)
  (for (_array_element_3 _array_index) _playercontrollerlist
    (Utilities|IsValid _array_element_3
      (:Is%20Not%20Valid
        (Utilities|Array|RemoveIndex _playercontrollerlist _array_index))))
  (for _array_element_4 _playercontrollerlist
    (Utilities|Array|Add (Variables|Default|GetPlayersTryingToJoin) _array_element_4)))

(event Custom|StopGame
  (for _array_element (Variables|Default|GetPlayerList)
    (Variables|/Game/Blueprints/MyCharacter2.MyCharacter2_C|Setenabled _array_element false)))

(event EventBeginPlay
  (Utilities|FlowControl|Delay 0.2)
  (Networking|SwitchHasAuthority
    (:Authority
      (bind _outactors (Actor|GetAllActorsOfClass "/Script/Engine.PlayerStart"))
      (Variables|Default|SetSpawnPoints _outactors)
      (bind _outactors_2 (Actor|GetAllActorsOfClass "/Game/Blueprints/WaitingZone.WaitingZone_C"))
      (Variables|Default|SetWaitingZonePoints _outactors_2)
      (bind _outactors_3 (Actor|GetAllActorsOfClass "/Game/Blueprints/QueueZone.QueueZone_C"))
      (Variables|Default|SetQueueZone (Utilities|Array|Get(acopy) _outactors_3))
      (Variables|/Game/Blueprints/QueueZone.QueueZone_C|SetWaitingZone (Utilities|Array|Get(acopy) _outactors_3) (Variables|Default|GetWaitingZonePoints))
      (bind _outactors_4 (Actor|GetAllActorsOfClass "/Game/Blueprints/Managers/GameManager.GameManager_C"))
      (Variables|Default|SetGameManager (Utilities|Array|Get(acopy) _outactors_4))
      (bind _outactors_5 (Actor|GetAllActorsOfClass "/Game/Blueprints/ResetManager.ResetManager_C"))
      (Variables|Default|SetResetManager (Utilities|Array|Get(acopy) _outactors_5))
      (Utilities|Time|SetTimerbyEvent (delegate Custom|OnPostLogin) 1.0 true))))

(event EventTick
  (params (DeltaSeconds :type Float%20%28single-precision%29)))

(event EventPostLogin
  (params (NewPlayer :type Player%20Controller%20Object%20Reference))
  (Networking|SwitchHasAuthority
    (:Authority
      (Utilities|Array|Add (Variables|Default|GetPlayersTryingToJoin) NewPlayer))))

(fn ConstructionScript)