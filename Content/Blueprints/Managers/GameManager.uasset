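; Game manager actor that switches between a cinematic waiting mode and gameplay, with helpers for countdown, join sound and cleanup.
; Cinematic mode shows a wait widget, plays victory music and picks a random cutscene, avoiding the previous one.
; Once both enter flags are set, TryToEnterInGame instead blends to the character camera with a fade and timeline-driven music fade-out.
; Tick interpolates platform heights toward the raised or lowered state toggled by PopPlateforme.
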(event Custom|PlayJoinSound
  (Default|PlayJoinSound (Variables|Default|GetCountDown)))

(event Custom|PopPlateforme
  (if (Variables|Default|GetplateformesUp)
    (Variables|Default|SetZPlateforme -3.6e+02)
    (Variables|Default|SetplateformesUp false)
    (else
      (Variables|Default|SetZPlateforme 0.0)
      (Variables|Default|SetplateformesUp true))))

(event Custom|ShowPressEnter
  (Utilities|FlowControl|DoOnce false
    (:Completed
      (bind _returnvalue (UserInterface|CreateWidget "/Game/Blueprints/Widgets/CinematicWaitWidget.CinematicWaitWidget_C" (Game|GetPlayerController 0)))
      (bind _output_get (Variables|Default|SetWaitWidget _returnvalue))
      (UserInterface|Viewport|AddtoViewport _output_get 0))))

(event Custom|HidePressEnter
  (Default|Hide (Variables|Default|GetWaitWidget)))

(event Custom|GoInCinematicMode
  (CallFunction|ResetWaitWidget)
  (if (not (Variables|/Game/Blueprints/CameraMovement.CameraMovement_C|GetGenericIsPlaying (Variables|Default|GetCameraMovement)))
    (Game|Player|SetViewTargetwithBlend (Game|GetPlayerController 0) (Variables|/Game/Blueprints/CameraMovement.CameraMovement_C|GetCamera (Variables|Default|GetCameraMovement)) 0.0 "VTBlend_Linear" 0.0 false)
    (CallFunction|TrytoEnterinGame)
    (Utilities|FlowControl|Delay 6.0)
    (Audio|Components|Audio|Play (Variables|Default|GetVictory_Cue) 0.0)))

(event Custom|Reset
  (Variables|Default|SetWantToEnter false)
  (Variables|Default|SetEnterPushed false))

(event Custom|ShowCountDown
  (Default|ShowTime (Variables|Default|GetCountDown)))

(event Custom|DestroyCameraAndPlayers
  (bind _outactors (Actor|GetAllActorsOfClass "/Game/Blueprints/Camera.Camera_C"))
  (for _array_element _outactors
    (Actor|DestroyActor _array_element)))

(event Custom|ResetWaitWidget
  (Utilities|FlowControl|DoOnce false) ; enters at Reset
)

(event Custom|FadeToGameEvent
  (Default|StopGeneric (Variables|Default|GetCameraMovement))
  (Utilities|FlowControl|Delay 0.6)
  (Game|Player|SetViewTargetwithBlend (Game|GetPlayerController 0) (Variables|/Game/Blueprints/MyCharacter2.MyCharacter2_C|GetCamera (Variables|Default|GetControlledCharacter)) 0.0 "VTBlend_Linear" 0.0 false)
  (Audio|Components|Audio|Play (Variables|Default|GetFadeFromBlack)))

(event Custom|TryToEnterInGame
  (bind _availablematinee (Variables|Default|GetAvailableMatinee))
  (if (and (Variables|Default|GetWantToEnter) (Variables|Default|GetEnterPushed))
    (CallFunction|FadetoGameEvent)
    (CallFunction|ShutDownVictoryFanfar)
    (else
      (Utilities|FlowControl|Delay 0.1)
      (Utilities|Array|Clear (Variables|Default|GetAvailableMatinee))
      (for _array_element (Variables|Default|GetCutScene)
        (if (!= _array_element (Variables|Default|GetSelectedMatinee))
          (Utilities|Array|Add _availablematinee _array_element)))
      (Utilities|Array|Shuffle _availablematinee)
      (Variables|Default|SetSelectedMatinee (Utilities|Array|Get(acopy) _availablematinee (Math|Random|RandomIntegerinRange 0 (- (Utilities|Array|Length _availablematinee) 1))))
      (Components|Animation|SetPosition (Variables|Default|GetSelectedMatinee) 0.0 true)
      (Audio|Components|Audio|Play (Variables|Default|GetSelectedMatinee)))))

(event Custom|ShutDownVictoryFanfar
  (bind _victory_cue (Variables|Default|GetVictory_Cue))
  (bind _newtrack_0 (Timeline|SoundPower PlayFromStart)
    (:Update
      (Audio|Components|Audio|SetVolumeMultiplier _victory_cue _newtrack_0 :!class /Script/Engine.AudioComponent))
    (:Finished
      (Audio|Components|Audio|Stop _victory_cue)
      (Audio|Components|Audio|SetVolumeMultiplier _victory_cue 0.75 :!class /Script/Engine.AudioComponent))))

(event EventBeginPlay
  (bind _victory_cue (Variables|Default|GetVictory_Cue))
  (Audio|Components|Audio|Stop _victory_cue)
  (Audio|Components|Audio|SetVolumeMultiplier _victory_cue 0.0 :!class /Script/Engine.AudioComponent)
  (Variables|Default|SetSelectedMatinee (Utilities|Array|Get(acopy) (Variables|Default|GetCutScene))))

(event EventActorBeginOverlap
  (params (OtherActor :type Actor%20Object%20Reference)))

(event EventTick
  (params (DeltaSeconds :type Float%20%28single-precision%29))
  (for (_array_element _array_index) (Variables|Default|GetPlateformesList)
    (Transformation|SetActorLocation _array_element (Math|Vector|MakeVector (.x (Transformation|GetActorLocation _array_element)) (.y (Transformation|GetActorLocation _array_element)) (Math|Interpolation|FInterpTo (.z (Transformation|GetActorLocation _array_element)) (+ (.z (Utilities|Array|Get(acopy) (Variables|Default|GetPlateformesPosition) _array_index)) (Variables|Default|GetZPlateforme)) (Utilities|Time|GetWorldDeltaSeconds) 1.0)) false true)))

(fn ConstructionScript)