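; Game instance that manages the front-end menus and LAN multiplayer sessions.
; A TransitionToState macro hides the current screen and updates the state; show events lazily create and reuse main menu, server list, loading and error widgets.
; Hosting creates a LAN session and opens FightMap as a listen server, while joining takes a server list result.
; Both show the loading screen and route failures to an error dialog that destroys the session.
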(event Custom|DestroySessionCaller
  (|DestroySession (Game|GetPlayerController 0)))

(event Custom|HostGame
  (CallFunction|ShowLoadingScreen)
  (|Session (Game|GetPlayerController 0) 8 true
    (:OnSuccess
      (Game|OpenLevel(byName) "FightMap" true "listen"))
    (:OnFailure
      (Utilities|DisplayErrorDialog "Failed to create session"))))

(event Custom|ShowMainMenu
  (Utilities|TransitiontoState "NewEnumerator1"
    (:SameState
      _)
    (:NewState
      _))
  (Utilities|IsValid (Variables|Default|GetMainMenu)
    (:Is%20Valid
      _)
    (:Is%20Not%20Valid
      (bind _returnvalue (UserInterface|CreateWidget "/Game/Blueprints/Widgets/MainMenuWidget.MainMenuWidget_C" (Game|GetPlayerController 0)))
      (Variables|Default|SetMainMenu _returnvalue)))
  (UserInterface|Viewport|AddtoViewport (Variables|Default|GetMainMenu) 0))

(event Custom|JoinFromServerList
  (params (Session :type Blueprint%20Session%20Result%20Structure))
  (CallFunction|ShowLoadingScreen)
  (|JoinSession (Game|GetPlayerController 0) Session
    (:OnFailure
      (Utilities|DisplayErrorDialog "Failed to join session"))))

(event Custom|ShowServerList
  (Utilities|TransitiontoState "NewEnumerator2"
    (:NewState
      (Utilities|IsValid (Variables|Default|GetServerList)
        (:Is%20Valid
          _)
        (:Is%20Not%20Valid
          (bind _returnvalue (UserInterface|CreateWidget "/Game/Blueprints/Widgets/ServerList.ServerList_C" (Game|GetPlayerController 0)))
          (Variables|Default|SetServerList _returnvalue)))
      (UserInterface|Viewport|AddtoViewport (Variables|Default|GetServerList) 0))))

(event Custom|ShowLoadingScreen
  (Utilities|TransitiontoState "NewEnumerator3"
    (:NewState
      (Utilities|IsValid (Variables|Default|GetLoadingScreen)
        (:Is%20Valid
          _)
        (:Is%20Not%20Valid
          (bind _returnvalue (UserInterface|CreateWidget "/Game/Blueprints/Widgets/LoadingScreen.LoadingScreen_C" (Game|GetPlayerController 0)))
          (Variables|Default|SetLoadingScreen _returnvalue)))
      (UserInterface|Viewport|AddtoViewport (Variables|Default|GetLoadingScreen) 0))))

(fn HideWidget
  (params (Widget :type Widget%20Object%20Reference))
  (Widget|RemovefromParent Widget))