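; QueueZone is a server-authoritative holding area that queues players until a waiting zone is free.
; AddPlayer, after a short delay, teleports the player to the spawn point, disables their Tirenabled flag and adds them to the list.
; A looping timer skips players in cinematics and passes the first eligible one to a free WaitingZone found by GetFreeWaitingZone, re-enabling Tirenabled and removing them from the list.
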(event Custom|AddPlayer
  (params (Player :type My%20Character%202%20Object%20Reference))
  (Networking|SwitchHasAuthority
    (:Authority
      (Utilities|IsValid Player
        (:Is%20Valid
          (Utilities|FlowControl|Delay 0.5)
          (Utilities|IsValid Player
            (:Is%20Valid
              (Default|ShowPressEnter Player)
              (Default|DisableShadows Player false)
              (Variables|/Game/Blueprints/MyCharacter2.MyCharacter2_C|Settirenabled Player false)
              (Variables|/Game/Blueprints/MyCharacter2.MyCharacter2_C|SetInWaitingZone Player true)
              (Utilities|Array|Add (Variables|Default|GetPlayerList) Player)
              (Transformation|SetActorLocation Player (Transformation|GetWorldLocation (Variables|Default|GetSpawnPoint)) false true))))))))

(event Custom|CheckPlayer
  (bind _waitingplayers (Variables|Default|GetWaitingPlayers))
  (bind _item (Utilities|Array|Get(acopy) _waitingplayers))
  (Networking|SwitchHasAuthority
    (:Authority
      (if (!= (Utilities|Array|Length (Variables|Default|GetPlayerList)) 0)
        (Utilities|Array|Clear (Variables|Default|GetWaitingPlayers))
        (for _array_element (Variables|Default|GetPlayerList)
          (Utilities|IsValid _array_element
            (:Is%20Valid
              (if (not (Variables|/Game/Blueprints/MyCharacter2.MyCharacter2_C|GetIsPlayingCinematic _array_element))
                (Utilities|Array|Add (Variables|Default|GetWaitingPlayers) _array_element)))))
        (if (!= (Utilities|Array|Length (Variables|Default|GetWaitingPlayers)) 0)
          (bind _waitingzone (Utilities|GetFreeWaitingZone)
            (:FreeZoneFound
              (Utilities|IsValid _item
                (:Is%20Valid
                  (Default|AddPlayer _waitingzone _item)
                  (Variables|/Game/Blueprints/MyCharacter2.MyCharacter2_C|Settirenabled _item true)
                  (Utilities|Array|RemoveItem (Variables|Default|GetPlayerList) _item))))))))))

(event EventBeginPlay
  (Utilities|Time|SetTimerbyEvent (delegate Custom|CheckPlayer) 0.2 true))

(event EventActorBeginOverlap
  (params (OtherActor :type Actor%20Object%20Reference)))

(event EventTick
  (params (DeltaSeconds :type Float%20%28single-precision%29)))

(fn ConstructionScript)