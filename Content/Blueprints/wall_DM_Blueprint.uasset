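; Destructible wall Blueprint that takes radius damage at given points through ApplyDamage and records each hit location.
; Shortly after BeginPlay it replays the recorded hits on the DestructibleComponent.
; On authority, a looping timer checks whether a box overlaps the destructible, nudging the box up and down on alternate checks.
; An overlap sets a timer for DestroyWall, which currently only prints a debug string.
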(event Custom|CheckDestructed
  (bind _box (Variables|Default|GetBox))
  (bind _box_2 (Variables|Default|GetBox))
  (bind _box_3 (Variables|Default|GetBox))
  (bind _returnvalue (Transformation|GetWorldLocation _box_2))
  (bind _returnvalue_2 (Transformation|GetWorldLocation _box_3))
  (if (Class|PrimitiveComponent|IsOverlappingComponent (Variables|Default|GetBox) (Variables|Default|GetDestructibleComponent))
    (Utilities|Time|SetTimerbyFunctionName 0 "DestroyWall" 5.0)
    (Development|PrintString "Hello"))
  (Utilities|FlowControl|FlipFlop
    (:A
      (Transformation|SetWorldLocation _box (Math|Vector|MakeVector (.x _returnvalue) (.y _returnvalue) (+ (.z _returnvalue) 0.1)) false false))
    (:B
      (Transformation|SetWorldLocation _box (Math|Vector|MakeVector (.x _returnvalue_2) (.y _returnvalue_2) (+ (.z _returnvalue_2) -0.1)) false false))))

(event Custom|ApplyDamage
  (params (Location :type Vector) (Damage :type Float%20%28single-precision%29))
  (Utilities|Array|Add (Variables|Default|GetHitLocation) Location)
  (Class|DestructibleComponent|ApplyRadiusDamage (Variables|Default|GetDestructibleComponent) Damage Location 32.0 1e+03 false))

(event EventBeginPlay
  (Utilities|FlowControl|Delay 0.5)
  (for _array_element (Variables|Default|GetHitLocation)
    (Class|DestructibleComponent|ApplyRadiusDamage (Variables|Default|GetDestructibleComponent) 1e+01 _array_element 32.0 1e+03 false))
  (Networking|SwitchHasAuthority
    (:Authority
      (Utilities|Time|SetTimerbyEvent (delegate Custom|CheckDestructed) 1.0 true))))

(event EventActorBeginOverlap
  (params (OtherActor :type Actor%20Object%20Reference)))

(event EventTick
  (params (DeltaSeconds :type Float%20%28single-precision%29)))

(fn ConstructionScript)

(fn DestroyWall
  (Development|PrintString "Coucou"))