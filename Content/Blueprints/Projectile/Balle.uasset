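; Bouncing bullet projectile that damages walls and characters, tinted with the shooter's color through a dynamic material.
; BeginPlay launches it along its direction, optionally ignores a wall collision channel and sets a lifespan.
; Server-authoritative bounces damage Mur or destructible walls and enforce a bounce limit, except on destructible-wall hits.
; Server-authoritative overlaps damage enabled characters, then hide the bullet, disable collision and shorten its lifespan.
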(event OnComponentBeginOverlap(SphereCollider)
  (params (OtherActor :type Actor%20Object%20Reference) (OtherComp :type Primitive%20Component%20Object%20Reference) (OtherBodyIndex :type Integer) (bFromSweep :type Boolean) (SweepResult :type Hit%20Result%20Structure%20%28by%20ref%29))
  (bind _asmy_character_2 (Utilities|Casting|CastToMyCharacter2 OtherActor))
  (Networking|SwitchHasAuthority
    (:Authority
      (if (and (!= 0 _asmy_character_2) (Variables|/Game/Blueprints/MyCharacter2.MyCharacter2_C|Getenabled _asmy_character_2))
        (Game|Damage|ApplyDamage _asmy_character_2 (* (Variables|Default|GetBaseDamage) (Variables|Default|GetDamageMultiplier)) 0 self "/Script/Engine.DamageType")
        (CallFunction|OnHit)))))

(event OnProjectileBounce(ProjectileMovement)
  (params (ImpactResult :type Hit%20Result%20Structure%20%28by%20ref%29) (ImpactVelocity :type Vector%20%28by%20ref%29 :default "0, 0, 0"))
  (bind (_bblockinghit _binitialoverlap _time _location _impactpoint _normal _impactnormal _physmat _hitactor) (Collision|BreakHitResult ImpactResult))
  (Networking|SwitchHasAuthority
    (:Authority
      (bind _result (Math|Integer|IncrementInt (Variables|Default|GetBounceNumber))
        (:%20%20
          (bind _asmur (Utilities|Casting|CastToMur _hitactor)
            (:then
              (Game|Damage|ApplyDamage _asmur (* (Variables|Default|GetBaseDamage) (Variables|Default|GetDamageMultiplier)) 0 self "/Script/Engine.DamageType")
              (if (> _result (Variables|Default|GetMaxBounceNumber)) :!label _label
                (Actor|DestroyActor)))
            (:CastFailed
              (bind _aswall_dm_blueprint (Utilities|Casting|CastTowall_DM_Blueprint _hitactor)
                (:then
                  (Default|ApplyDamage _aswall_dm_blueprint _impactpoint 1e+01))
                (:CastFailed
                  (goto _label))))))))))

(event Custom|OnHit
  (Collision|SetActorEnableCollision false)
  (Rendering|SetActorHiddenInGame true)
  (Actor|SetLifeSpan 1.0))

(event Custom|UpdatePosition
  (params (Position :type Vector)))

(event EventBeginPlay
  (bind _tireur (Variables|Default|GetTireur))
  (bind _color (Variables|/Game/Blueprints/MyCharacter.MyCharacter_C|GetColor _tireur))
  (Transformation|SetActorLocation (Transformation|GetActorLocation) false false)
  (Variables|/Script/Engine.MovementComponent|SetVelocity (Variables|Default|GetProjectileMovement) (* (Variables|Default|GetDirection) (Variables|Default|Getspeed)))
  (if (Variables|Default|GetthroughWalls)
    (Collision|SetCollisionResponsetoChannel (Variables|Default|GetSphereCollider) "ECC_GameTraceChannel5" "ECR_Ignore"))
  (Actor|SetLifeSpan 1e+01)
  (Utilities|IsValid _tireur
    (:Is%20Valid
      (Rendering|Material|SetVectorParameterValue (Variables|Default|GetmatBalle) "Couleur" (Math|Color|MakeColor (* (.r _color) 3.0) (* (.g _color) 3.0) (* (.b _color) 3.0)) :!class /Script/Engine.MaterialInstanceDynamic))))

(event Collision|EventActorBeginOverlap
  (params (OtherActor :type Actor%20Object%20Reference)))

(event EventTick
  (params (DeltaSeconds :type Float%20%28single-precision%29)))

(fn ConstructionScript
  (bind _returnvalue (Rendering|Material|CreateDynamicMaterialInstance (Variables|Default|GetBalleMesh) 0 "/Game/Effects/Materials/MatBalle.MatBalle" :!class /Script/Engine.PrimitiveComponent))
  (Variables|Default|SetmatBalle _returnvalue))