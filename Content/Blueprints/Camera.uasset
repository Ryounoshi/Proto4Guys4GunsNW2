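; Player camera that follows Joueur0 in the waiting zone, otherwise frames active MyCharacter2 players, with an in-world HUD for Joueur0.
; UpdateView rebuilds the player list, dropping waiting players, and applies the player color.
; Tick eases toward a point halfway between world origin and the players' bounding center, scaling arm length by the square root of their maximum separation.
; It also draws debug-trace aim lines and updates score, XP, level, penalty and control icon.
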(event Custom|UpdateView
  (Utilities|FlowControl|Delay 0.2)
  (bind _outactors (Actor|GetAllActorsOfClass "/Game/Blueprints/MyCharacter2.MyCharacter2_C"))
  (bind _output_get (Variables|Default|SetcharList _outactors))
  (for _array_element _output_get
    (if (Variables|/Game/Blueprints/MyCharacter2.MyCharacter2_C|GetInWaitingZone _array_element)
      (Utilities|Array|RemoveItem _output_get _array_element)))
  (for _array_element_2 _output_get
    (Default|RefreshTextandColor _array_element_2))
  (Variables|Default|Setloading false)
  (bind _returnvalue (Rendering|Material|CreateDynamicMaterialInstance (Variables|Default|GetPlayerColor) 0 "/Game/Effects/Materials/DynamicColor.DynamicColor" :!class /Script/Engine.PrimitiveComponent))
  (Rendering|Material|SetVectorParameterValue _returnvalue "Color" (Variables|/Game/Blueprints/MyCharacter2.MyCharacter2_C|GetColor (Variables|Default|GetJoueur0)) :!class /Script/Engine.MaterialInstanceDynamic))

(event EventBeginPlay
  ;[1 1 1] Init
)

(event Collision|EventActorBeginOverlap
  (params (OtherActor :type Actor%20Object%20Reference)))

(event EventTick
  (params (DeltaSeconds :type Float%20%28single-precision%29))
  (bind _returnvalue (Utilities|Time|GetWorldDeltaSeconds))
  (bind _xpbar (Variables|Default|GetxpBar))
  (bind _joueur0 (Variables|Default|GetJoueur0))
  (bind _xpbar_2 (Variables|Default|GetxpBar))
  (bind _controltype (Variables|Default|GetControlType))
  (bind _experience (Variables|/Game/Blueprints/MyCharacter2.MyCharacter2_C|GetExperience _joueur0))
  (if (not (Variables|Default|Getloading))
    (Utilities|FlowControl|Sequence
      (:then_0
        (if (Variables|/Game/Blueprints/MyCharacter2.MyCharacter2_C|GetInWaitingZone (Variables|Default|GetJoueur0))
          (Transformation|SetActorLocation (Math|Interpolation|VInterpTo (Transformation|GetActorLocation) (Transformation|GetActorLocation (Variables|Default|GetJoueur0)) (Utilities|Time|GetWorldDeltaSeconds) (Variables|Default|GetinterpSpeed)) false false)
          (else
            (Variables|Default|SetXmax -1e+04)
            (Variables|Default|SetYmax -1e+04)
            (Variables|Default|SetYmin 1e+04)
            (Variables|Default|SetXmin 1e+04)
            (Variables|Default|Setdistmax 0.0)
            (for _array_element (Variables|Default|GetcharList)
              (Utilities|IsValid _array_element
                (:Is%20Valid
                  (for _array_element_2 (Variables|Default|GetcharList)
                    (Utilities|IsValid _array_element_2
                      (:Is%20Valid
                        (Variables|Default|Setdistmax (Math|Float|Max(Float) (Math|Vector|VectorLength (- (Transformation|GetActorLocation _array_element) (Transformation|GetActorLocation _array_element_2))) (Variables|Default|Getdistmax)))
                        (Variables|Default|SetXmax (Math|Float|Max(Float) (.x (Transformation|GetActorLocation _array_element)) (.x (Transformation|GetActorLocation _array_element_2)) (Variables|Default|GetXmax)))
                        (Variables|Default|SetYmax (Math|Float|Max(Float) (.y (Transformation|GetActorLocation _array_element)) (.y (Transformation|GetActorLocation _array_element_2)) (Variables|Default|GetYmax)))
                        (Variables|Default|SetYmin (Math|Float|Min(Float) (.y (Transformation|GetActorLocation _array_element)) (.y (Transformation|GetActorLocation _array_element_2)) (Variables|Default|GetYmin)))
                        (Variables|Default|SetXmin (Math|Float|Min(Float) (.x (Transformation|GetActorLocation _array_element)) (.x (Transformation|GetActorLocation _array_element_2)) (Variables|Default|GetXmin)))))))))
            ;[1 1 1] Follow Players
            (Transformation|SetActorLocation (Math|Vector|MakeVector (.x (Math|Interpolation|VInterpTo (Transformation|GetActorLocation) (/ (+ (Math|Vector|MakeVector (/ (+ (Variables|Default|GetXmax) (Variables|Default|GetXmin)) 2.0) (/ (+ (Variables|Default|GetYmax) (Variables|Default|GetYmin)) 2.0) 0.0) "0, 0, 0") 2.0) (Utilities|Time|GetWorldDeltaSeconds) (Variables|Default|GetinterpSpeed))) (.y (Math|Interpolation|VInterpTo (Transformation|GetActorLocation) (/ (+ (Math|Vector|MakeVector (/ (+ (Variables|Default|GetXmax) (Variables|Default|GetXmin)) 2.0) (/ (+ (Variables|Default|GetYmax) (Variables|Default|GetYmin)) 2.0) 0.0) "0, 0, 0") 2.0) (Utilities|Time|GetWorldDeltaSeconds) (Variables|Default|GetinterpSpeed))) (.z (Math|Interpolation|VInterpTo (Transformation|GetActorLocation) (/ (+ (Math|Vector|MakeVector (/ (+ (Variables|Default|GetXmax) (Variables|Default|GetXmin)) 2.0) (/ (+ (Variables|Default|GetYmax) (Variables|Default|GetYmin)) 2.0) 0.0) "0, 0, 0") 2.0) (Utilities|Time|GetWorldDeltaSeconds) (Variables|Default|GetinterpSpeed)))) false false)
            ;;[1 1 1] Zoom
            (Variables|/Script/Engine.SpringArmComponent|SetTargetArmLength (Variables|Default|GetSpringArm) (Math|Interpolation|FInterpTo (Variables|/Script/Engine.SpringArmComponent|GetTargetArmLength (Variables|Default|GetSpringArm)) (* (Math|Float|Clamp(Float) (Math|Float|Sqrt (/ (Variables|Default|Getdistmax) 3.2e+02)) 2.0 3e+03) (Variables|Default|GetarmLenght)) (Utilities|Time|GetWorldDeltaSeconds) 6.0)))))
      (:then_1
        ;[1 1 1] Players Score
        (Rendering|Components|TextRender|SetText (Variables|Default|GetScore1) (Utilities|Text|ToText(Integer) (Variables|/Game/Blueprints/MyCharacter2.MyCharacter2_C|Getscore (Variables|Default|GetJoueur0)))))
      (:then_2
        (if (not (Variables|/Game/Blueprints/MyCharacter2.MyCharacter2_C|GetInWaitingZone (Variables|Default|GetJoueur0)))
          ;[1 1 1] Visée des joueurs
          (for _array_element_3 (Variables|Default|GetcharList)
            (Utilities|IsValid _array_element_3
              (:Is%20Valid
                (if (Variables|/Game/Blueprints/MyCharacter2.MyCharacter2_C|Getenabled _array_element_3)
                  (bind _outhit (Collision|LineTraceByChannel (Math|Vector|MakeVector (.x (Transformation|GetActorLocation _array_element_3)) (.y (Transformation|GetActorLocation _array_element_3)) (- (.z (Transformation|GetActorLocation _array_element_3)) 2e+01)) (Math|Vector|MakeVector (.x (+ (Math|Vector|MakeVector (.x (Transformation|GetActorLocation _array_element_3)) (.y (Transformation|GetActorLocation _array_element_3)) (.z (Transformation|GetActorLocation _array_element_3))) (* (Variables|/Game/Blueprints/MyCharacter2.MyCharacter2_C|GetDirTir _array_element_3) 1e+04))) (.y (+ (Math|Vector|MakeVector (.x (Transformation|GetActorLocation _array_element_3)) (.y (Transformation|GetActorLocation _array_element_3)) (.z (Transformation|GetActorLocation _array_element_3))) (* (Variables|/Game/Blueprints/MyCharacter2.MyCharacter2_C|GetDirTir _array_element_3) 1e+04))) (- (.z (+ (Math|Vector|MakeVector (.x (Transformation|GetActorLocation _array_element_3)) (.y (Transformation|GetActorLocation _array_element_3)) (.z (Transformation|GetActorLocation _array_element_3))) (* (Variables|/Game/Blueprints/MyCharacter2.MyCharacter2_C|GetDirTir _array_element_3) 1e+04))) 2e+01)) "TraceTypeQuery1" false (Utilities|Array|MakeArray _array_element_3) "ForOneFrame"))))))))
      (:then_3
        (if (Variables|/Game/Blueprints/MyCharacter2.MyCharacter2_C|GetUseKeyBoard (Variables|Default|GetJoueur0))
          (Rendering|Material|SetMaterial _controltype 0 "/Game/Effects/Materials/mouse_Mat.mouse_Mat")
          (else
            (Rendering|Material|SetMaterial _controltype 0 "/Game/Effects/Materials/gamepad_Mat.gamepad_Mat"))))
      (:then_4
        ;[1 1 1] Infos Diverses
        (Rendering|Components|TextRender|SetText (Variables|Default|Getxp) (Utilities|Text|ToText(Float) (Variables|/Game/Blueprints/MyCharacter2.MyCharacter2_C|GetExperience (Variables|Default|GetJoueur0)) "HalfToEven"))
        (Rendering|Components|TextRender|SetText (Variables|Default|GetLevel) (Utilities|Text|ToText(Integer) (Variables|/Game/Blueprints/MyCharacter2.MyCharacter2_C|GetLevel (Variables|Default|GetJoueur0))))
        (Rendering|Components|TextRender|SetText (Variables|Default|GetPenality) (Utilities|Text|ToText(Float) (Variables|/Game/Blueprints/MyCharacter2.MyCharacter2_C|GetPenalityPoints (Variables|Default|GetJoueur0)) "HalfToEven")))
      (:then_5
        ;[1 1 1] Barre d'xp
        (Transformation|SetRelativeTransform (Variables|Default|GetxpBar) (Math|Transform|MakeTransform (Math|Vector|MakeVector 4e+01 (Math|Interpolation|FInterpTo (.y (Variables|/Script/Engine.SceneComponent|GetRelativeLocation _xpbar)) (+ -39.0 (/ _experience 33.333)) _returnvalue 12.0) 17.0) "0, 0, 0" (Math|Vector|MakeVector 0.001 (Math|Interpolation|FInterpTo (.y (Variables|/Script/Engine.SceneComponent|GetRelativeScale3D _xpbar)) (* 0.06 (Math|Float|Clamp(Float) (/ _experience 1e+02) 0.001 1e+06)) _returnvalue 12.0) 0.01)) false false))
      (:then_6
        ;[1 1 1] Barres d'xp (visibility)
        (if (<= _experience 0.0)
          (Rendering|SetVisibility _xpbar_2 false true)
          (else
            (Rendering|SetVisibility _xpbar_2 true true))))
      (:then_7
        ;[1 1 1] Option
        (Rendering|SetVisibility (Variables|Default|GetHaveOption) (Variables|/Game/Blueprints/MyCharacter2.MyCharacter2_C|GethaveOption (Variables|Default|GetJoueur0)) false)))))

(fn ConstructionScript
  (Variables|/Script/Engine.SpringArmComponent|SetTargetArmLength (Variables|Default|GetSpringArm) (Variables|Default|GetarmLenght))
  (Transformation|SetRelativeRotation (Variables|Default|GetSpringArm) (Math|Rotator|MakeRotator 0.0 (Variables|Default|Getarmrotation) 0.0) false false)
  (Variables|/Script/Engine.CameraComponent|SetOrthoWidth (Variables|Default|GetCamera) (Variables|Default|Getdistance)))