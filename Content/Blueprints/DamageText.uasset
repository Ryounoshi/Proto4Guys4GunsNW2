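; DamageText is a short-lived actor that shows a floating, animated text popup, by its name for damage numbers.
; The construction script sets the TextRender's text and color from Value and Color and creates a dynamic unlit material instance for fading.
; On BeginPlay, the Movement timeline drives an offset along the up vector and Y with slight random variation, plus scale and opacity, then destroys the actor.
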(event EventBeginPlay
  (bind _textrender (Variables|Default|GetTextRender))
  (Components|Timeline|SetPlayRate (Variables|Default|GetMovement) 0.8)
  (Variables|Default|SetZRandomVariationMultiplier (Math|Random|RandomFloatinRange 0.95 1.05))
  (bind _output_get (Variables|Default|SetYRandVariation (Math|Random|RandomFloatinRange 0.6 0.8)))
  (bind (_direction _zvalue _yvalue _alphavalue _yscale _xscale) (Timeline|Movement Play)
    (:Update
      (Transformation|SetRelativeLocation _textrender (+ (* (Math|Vector|GetUpVector _textrender) (* (Variables|Default|GetZRandomVariationMultiplier) (* _zvalue 2.5e+02))) (Math|Vector|MakeVector 0.0 (* _yvalue (* (Variables|Default|GetYRandVariation) 1.6e+02)) 0.0)) false false)
      (Rendering|Material|SetScalarParameterValue (Variables|Default|GetMat) "Opacity" _alphavalue :!class /Script/Engine.MaterialInstanceDynamic)
      (Rendering|Components|TextRender|SetYScale _textrender _yscale)
      (Rendering|Components|TextRender|SetXScale _textrender _xscale))
    (:Finished
      (Actor|DestroyActor))))

(event EventActorBeginOverlap
  (params (OtherActor :type Actor%20Object%20Reference)))

(event EventTick
  (params (DeltaSeconds :type Float%20%28single-precision%29)))

(fn ConstructionScript
  (bind _textrender (Variables|Default|GetTextRender))
  (bind _returnvalue (Rendering|Material|CreateDynamicMaterialInstance _textrender 0 "/Game/Effects/Materials/TextUnlite.TextUnlite" :!class /Script/Engine.PrimitiveComponent))
  (Variables|Default|SetMat _returnvalue)
  (Rendering|Components|TextRender|SetText _textrender (Variables|Default|GetValue))
  (Rendering|Components|TextRender|SetTextRenderColor _textrender (Math|Conversions|ToColor(LinearColor) (Variables|Default|GetColor))))