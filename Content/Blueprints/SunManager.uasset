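; SunManager drives a day-night cycle by pitching the Sun actor and refreshing the sky sphere, skylight intensity and emissive power parameter.
; Authority advances Rotation every other tick and stores ActualRotation, which remotes apply to their sun.
; Nested FlipFlops throttle a slower check that varies sun speed by angle and hides its light at night.
; Rotation resets when the sun nears RefPoint, its starting orientation.
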(event EventBeginPlay
  (Transformation|SetActorRotation (Variables|Default|GetSun) (Variables|Default|GetRefPoint))
  (Default|UpdateSunDirection (Variables|Default|GetSkySphere)))

(event EventActorBeginOverlap
  (params (OtherActor :type Actor%20Object%20Reference)))

(event EventTick
  (params (DeltaSeconds :type Float%20%28single-precision%29))
  (bind _sun (Variables|Default|GetSun))
  (Networking|SwitchHasAuthority
    (:Authority
      (Utilities|FlowControl|FlipFlop
        (:A
          (bind _output_get (Variables|Default|SetRotation (+ (Variables|Default|GetRotation) (* (Utilities|Time|GetWorldDeltaSeconds) (* (Variables|Default|GetVitesseDuSoleil) (Variables|Default|GetSunSpeed))))))
          (if (Math|Rotator|Equal(Rotator) (Variables|Default|GetRefPoint) (Transformation|GetActorRotation (Variables|Default|GetSun)) 1.0)
            (Variables|Default|SetRotation 0.0))
          (Class|Actor|AddActorWorldRotation _sun (Math|Rotator|MakeRotator 0.0 (* (Utilities|Time|GetWorldDeltaSeconds) (* (Variables|Default|GetVitesseDuSoleil) (Variables|Default|GetSunSpeed))) 0.0))
          (Variables|Default|SetActualRotation (Transformation|GetActorRotation _sun))
          (Default|UpdateSunDirection (Variables|Default|GetSkySphere))
          (Rendering|Components|Light|SetIntensity (Variables|/Script/Engine.SkyLight|GetLightComponent (Variables|Default|GetSkyLight)) (+ (/ (Math|Float|Clamp(Float) (- (Math|Float|Absolute(Float) (- 1.8e+02 _output_get)) 9e+01) 0.0 1.8e+02) 9e+01) 0.4))
          (Rendering|Material|SetScalarParameterValue "/Game/Effects/Materials/EmisivePower.EmisivePower" "Power" (+ (/ (Math|Float|Clamp(Float) (- (Math|Float|Absolute(Float) (- 1.8e+02 _output_get)) 9e+01) 0.0 1.8e+02) 9e+01) (Variables|Default|GetGlowPower)) :!class /Script/Engine.KismetMaterialLibrary)
          (Utilities|FlowControl|FlipFlop
            (:A
              (Utilities|FlowControl|FlipFlop
                (:A
                  (Utilities|FlowControl|FlipFlop
                    (:A
                      (if (and (> (Variables|Default|GetRotation) 0.0) (<= (Variables|Default|GetRotation) 9e+01))
                        (Variables|Default|SetVitesseDuSoleil (+ 1.0 (/ (- 8e+01 (Variables|Default|GetRotation)) 3e+01)))
                        (Rendering|SetVisibility (Variables|/Script/Engine.Light|GetLightComponent (Variables|Default|GetSun)) true false)
                        (elif (and (>= (Variables|Default|GetRotation) 1e+02) (< (Variables|Default|GetRotation) 1.2e+02))
                          (Variables|Default|SetVitesseDuSoleil 3.0)
                          (Rendering|SetVisibility (Variables|/Script/Engine.Light|GetLightComponent (Variables|Default|GetSun)) false false)
                          (elif (and (>= (Variables|Default|GetRotation) 2.7e+02) (< (Variables|Default|GetRotation) 3.6e+02))
                            (Variables|Default|SetVitesseDuSoleil (+ (/ (- (Variables|Default|GetRotation) 2.8e+02) 3e+01) 1.0))
                            (Rendering|SetVisibility (Variables|/Script/Engine.Light|GetLightComponent (Variables|Default|GetSun)) true false)))))))))))))
    (:Remote
      (Transformation|SetActorRotation (Variables|Default|GetSun) (Variables|Default|GetActualRotation))
      (Rendering|Components|Light|SetIntensity (Variables|/Script/Engine.SkyLight|GetLightComponent (Variables|Default|GetSkyLight)) (+ (/ (Math|Float|Clamp(Float) (- (Math|Float|Absolute(Float) (- 1.8e+02 (Variables|Default|GetRotation))) 9e+01) 0.0 1.8e+02) 9e+01) 0.4))
      (Rendering|Material|SetScalarParameterValue "/Game/Effects/Materials/EmisivePower.EmisivePower" "Power" (+ (/ (Math|Float|Clamp(Float) (- (Math|Float|Absolute(Float) (- 1.8e+02 (Variables|Default|GetRotation))) 9e+01) 0.0 1.8e+02) 9e+01) (Variables|Default|GetGlowPower)) :!class /Script/Engine.KismetMaterialLibrary)
      (Default|UpdateSunDirection (Variables|Default|GetSkySphere)))))

(fn ConstructionScript)