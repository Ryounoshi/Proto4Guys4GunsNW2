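; Spline actor Blueprint that builds a chain of spline mesh components along its Spline component.
; CreateMesh loops over the spline points, adds and attaches a SplineMeshComponent for each, and bends it to the next point using world-space locations and tangents.
; The construction script is empty and the event stubs are disabled, so nothing in this file calls CreateMesh.
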(event EventBeginPlay)

(event EventActorBeginOverlap
  (params (OtherActor :type Actor%20Object%20Reference)))

(event EventTick
  (params (DeltaSeconds :type Float%20%28single-precision%29)))

(fn ConstructionScript)

(fn CreateMesh
  (bind _spline (Variables|Default|GetSpline))
  (for _index (range 0 (Spline|GetNumberOfSplinePoints (Variables|Default|GetSpline)))
    (bind _returnvalue (AddComponent|AddSplineMeshComponent true (Transformation|GetActorTransform)))
    (Class|SceneComponent|Attachto _returnvalue (VehicleSound|GetRootComponent) "None" "KeepRelativeOffset" true)
    (SplineMesh|SetStartandEnd _returnvalue (.Location (Spline|GetLocationandTangentatSplinePoint _spline _index "World")) (.Tangent (Spline|GetLocationandTangentatSplinePoint _spline _index "World")) (.Location (Spline|GetLocationandTangentatSplinePoint _spline (+ _index 1) "World")) (.Tangent (Spline|GetLocationandTangentatSplinePoint _spline (+ _index 1) "World")) :!class /Script/Engine.SplineMeshComponent)))