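; OptionManager is an actor that periodically spawns Option pickup actors onto the board during play.
; On BeginPlay the server starts a looping RespawnTime timer, and each tick spawns an Option only while NbOptionOnBoard is below MaxOptionsOnBoard.
; Each Option appears at a random X/Y within a square centred on the origin, raised and scaled up, and receives a reference to this manager.
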(event Custom|SpawnOption_Event
  (Networking|SwitchHasAuthority
    (:Authority
      (if (< (Variables|Default|GetnbOptionOnBoard) (Variables|Default|GetMaxOptionsOnBoard))
        (Game|SpawnActorfromClass "/Game/Blueprints/Options/Option.Option_C" (Math|Transform|MakeTransform (Math|Vector|MakeVector (- (Math|Random|RandomFloatinRange 0.0 3.4e+03) 1.7e+03) (- (Math|Random|RandomFloatinRange 0.0 3.4e+03) 1.7e+03) 5e+02) "0, 0, 0" "2.000000,2.000000,2.000000") "Undefined" 0 self 0)))))

(event EventBeginPlay
  (Networking|SwitchHasAuthority
    (:Authority
      (Utilities|Time|SetTimerbyEvent (delegate Custom|SpawnOption_Event) (Variables|Default|GetRespawnTime) true))))

(event EventActorBeginOverlap
  (params (OtherActor :type Actor%20Object%20Reference)))

(event EventTick
  (params (DeltaSeconds :type Float%20%28single-precision%29)))

(fn ConstructionScript)