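; A pickup actor that grants a random Option to the first MyCharacter2 without one that overlaps its sphere.
; The construction script rolls an option, but on BeginPlay the authority rerolls it between two enum values and increments the OptionManager's on-board count.
; Authority-side pickup hands over the option, decrements that count, plays a ring sound and destroys the actor.
; Tick spins the sphere while holding the question mark at a fixed world rotation.
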(event OnComponentBeginOverlap(Sphere)
  (params (OtherActor :type Actor%20Object%20Reference) (OtherComp :type Primitive%20Component%20Object%20Reference) (OtherBodyIndex :type Integer) (bFromSweep :type Boolean) (SweepResult :type Hit%20Result%20Structure%20%28by%20ref%29))
  (bind _asmy_character_2 (Utilities|Casting|CastToMyCharacter2 OtherActor))
  (CallFunction|PickOption _asmy_character_2))

(event Custom|PickOption
  (params (Character :type My%20Character%202%20Object%20Reference))
  (Networking|SwitchHasAuthority
    (:Authority
      (if (not (Variables|/Game/Blueprints/MyCharacter2.MyCharacter2_C|GethaveOption Character))
        (Variables|/Game/Blueprints/MyCharacter2.MyCharacter2_C|Setoption Character (Variables|Default|Getoption))
        (Variables|/Game/Blueprints/MyCharacter2.MyCharacter2_C|SethaveOption Character true)
        (Math|Integer|DecrementInt (Variables|/Game/Blueprints/Options/OptionManager.OptionManager_C|GetnbOptionOnBoard (Variables|Default|GetOptionManager))
          (:%20%20
            (CallFunction|PlayPickSound)
            (Actor|DestroyActor)))))))

(event Custom|PlayPickSound
  (Audio|PlaySound2D "/Game/Son/Sonic_Ring_Sound_Effect.Sonic_Ring_Sound_Effect"))

(event EventBeginPlay
  (Networking|SwitchHasAuthority
    (:Authority
      (Math|Integer|IncrementInt (Variables|/Game/Blueprints/Options/OptionManager.OptionManager_C|GetnbOptionOnBoard (Variables|Default|GetOptionManager))
        (:%20%20
          (switch int (Math|Random|RandomIntegerinRange 0 1)
            (:0
              (Variables|Default|Setoption "NewEnumerator0"))
            (:1
              (Variables|Default|Setoption "NewEnumerator4"))))))))

(event EventActorBeginOverlap
  (params (OtherActor :type Actor%20Object%20Reference)))

(event EventTick
  (params (DeltaSeconds :type Float%20%28single-precision%29))
  (bind _sphere (Variables|Default|GetSphere))
  (bind _questionmark (Variables|Default|GetquestionMark))
  (bind _output_get (Variables|Default|Setrotation (+ (Variables|Default|Getrotation) 0.5)))
  (Transformation|SetWorldRotation _sphere (Math|Rotator|MakeRotator 0.0 0.0 (Math|Interpolation|FInterpTo (.yaw (Transformation|GetWorldRotation _sphere)) _output_get 0.0 0.0)) false false)
  (Utilities|IsValid _questionmark
    (:Is%20Valid
      (Transformation|SetWorldRotation _questionmark "90.000000,180.000000, 0" false false))))

(fn ConstructionScript
  (Variables|Default|Setoption (Utilities|Select :Index (Math|Random|RandomIntegerinRange 0 2) :Option%200 "NewEnumerator0" :Option%201 "NewEnumerator1" :Option%202 "NewEnumerator2")))