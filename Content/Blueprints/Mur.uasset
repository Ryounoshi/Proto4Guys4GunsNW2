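; Destructible wall that takes damage, sinks underground when destroyed and rebuilds itself after a random delay.
; Damage is handled on authority: grenades scale by horizontal distance, other hits remove one life, and brick materials swap to show remaining health.
; At zero life the mesh shatters through radius damage, then later resets and rises to its initial position.
; Tick-fed gates drive both interpolated movements, while DestroyFast teleports an already destroyed wall below ground.
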(event Custom|DetruireMur_Event
  (bind _returnvalue (Utilities|Time|GetWorldDeltaSeconds))
  (bind _returnvalue_2 (Transformation|GetActorLocation))
  (bind _returnvalue_3 (Math|Interpolation|FInterpTo (.z _returnvalue_2) -2e+02 _returnvalue 4.0))
  (Collision|SetCollisionEnabled (Variables|Default|GetBoxCollider) "QueryAndPhysics")
  (Class|DestructibleComponent|ApplyRadiusDamage (Variables|Default|GetDestructibleComponent) 1e+01 (Transformation|GetActorLocation) 2e+02 1.0 true)
  (Utilities|FlowControl|Delay 0.2)
  (Utilities|FlowControl|Gate true) ; enters at Open
)

(event Custom|ConstruireMur_Event
  (bind _returnvalue (Utilities|Time|GetWorldDeltaSeconds))
  (bind _returnvalue_2 (Transformation|GetActorLocation))
  (bind _initiallocation (Variables|Default|GetInitialLocation))
  (bind _returnvalue_3 (Math|Interpolation|FInterpTo (.z _returnvalue_2) (.z _initiallocation) _returnvalue 3.0))
  (Variables|Default|Setlife 1e+01)
  (Class|DestructibleComponent|SetDestructibleMesh (Variables|Default|GetDestructibleComponent) "/Game/Mesh/mumu_DM.mumu_DM")
  (Collision|SetCollisionEnabled (Variables|Default|GetBoxCollider) "QueryAndPhysics")
  (CallFunction|UpdateMat)
  (Utilities|FlowControl|Gate true) ; enters at Open
)

(event Custom|UpdateMat
  (bind _life (Variables|Default|Getlife))
  (bind _destructiblecomponent (Variables|Default|GetDestructibleComponent))
  (if (>= _life 7.0)
    (Rendering|Material|SetMaterial _destructiblecomponent 0 "/Game/Effects/Materials/Brick_BathStone.Brick_BathStone")
    (elif (and (< _life 7.0) (>= _life 3.0))
      (Rendering|Material|SetMaterial _destructiblecomponent 0 "/Game/Effects/Materials/Brick_BathStone_Half_Destroyed.Brick_BathStone_Half_Destroyed")
      (else
        (Rendering|Material|SetMaterial _destructiblecomponent 0 "/Game/Effects/Materials/Brick_BathStone_Destroyed.Brick_BathStone_Destroyed")))))

(event Custom|DestroyFast
  (bind _returnvalue (Transformation|GetActorLocation))
  (if (Variables|Default|Getdestroyed)
    (Transformation|SetActorLocation (Math|Vector|MakeVector (.x _returnvalue) (.y _returnvalue) -2e+02) false true)))

(event Game|Damage|EventAnyDamage
  (params (Damage :type Float%20%28single-precision%29) (DamageType :type Damage%20Type%20Object%20Reference) (InstigatedBy :type Controller%20Object%20Reference) (DamageCauser :type Actor%20Object%20Reference))
  (bind _returnvalue (Transformation|GetActorLocation))
  ;[0.3 0.3 1] Handle Damage
  (Networking|SwitchHasAuthority
    (:Authority
      (if (Variables|Default|GetcanbeDestroyed)
        (if (not (Variables|Default|Getdestroyed))
          (bind _asgrenade (Utilities|Casting|CastToGrenade DamageCauser)
            (:then
              (Variables|Default|Setlife (- (Variables|Default|Getlife) (- 1e+01 (/ (Math|Vector|VectorLength (- (Math|Vector|MakeVector (.x _returnvalue) (.y _returnvalue) 0.0) (Math|Vector|MakeVector (.x (Transformation|GetActorLocation _asgrenade)) (.y (Transformation|GetActorLocation _asgrenade)) 0.0))) 1e+02)))))
            (:CastFailed
              (Math|Float|DecrementFloat (Variables|Default|Getlife)
                (:%20%20
                  _))))
          (CallFunction|UpdateMat)
          (if (<= (Variables|Default|Getlife) 0.0)
            (Variables|Default|Setdestroyed true)
            (CallFunction|DetruireMurEvent)
            (Utilities|FlowControl|Delay (Math|Random|RandomFloatinRange 5.0 2e+01))
            (CallFunction|ConstruireMurEvent)))))))

(event EventBeginPlay
  (Variables|Default|SetInitialLocation (Transformation|GetActorLocation)))

(event Collision|EventActorBeginOverlap
  (params (OtherActor :type Actor%20Object%20Reference)))

(event EventTick
  (params (DeltaSeconds :type Float%20%28single-precision%29))
  (bind _returnvalue (Utilities|Time|GetWorldDeltaSeconds))
  (bind _returnvalue_2 (Utilities|Time|GetWorldDeltaSeconds))
  (bind _returnvalue_3 (Transformation|GetActorLocation))
  (bind _returnvalue_4 (Transformation|GetActorLocation))
  (bind _initiallocation (Variables|Default|GetInitialLocation))
  (bind _returnvalue_5 (Math|Interpolation|FInterpTo (.z _returnvalue_4) (.z _initiallocation) _returnvalue 3.0))
  (bind _returnvalue_6 (Math|Interpolation|FInterpTo (.z _returnvalue_3) -2e+02 _returnvalue_2 4.0))
  (Utilities|FlowControl|Sequence
    (:then_0
      (Utilities|FlowControl|Gate true :!label _label
        (:Exit
          (Transformation|SetActorLocation (Math|Vector|MakeVector (.x _returnvalue_3) (.y _returnvalue_3) _returnvalue_6) false false)
          (if (<= _returnvalue_6 -199.0)
            (goto _label Close)))))
    (:then_1
      (Utilities|FlowControl|Gate true :!label _label_2
        (:Exit
          (Transformation|SetActorLocation (Math|Vector|MakeVector (.x _returnvalue_4) (.y _returnvalue_4) _returnvalue_5) false false)
          (if (>= _returnvalue_5 (- (.z _initiallocation) 0.5))
            (Variables|Default|Setdestroyed false)
            (goto _label_2 Close)))))))

(fn ConstructionScript)