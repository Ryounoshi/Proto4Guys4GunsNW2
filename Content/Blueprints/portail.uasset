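; Portal actor that teleports any actor overlapping its static mesh to a randomly chosen linked portal, provided this portal is enabled.
; It picks the destination from the OtherPortail array and moves the actor to that portal's X and Y, keeping the actor's own Z.
; The destination is disabled for a one-frame delay around the teleport, then re-enabled only if the actor is still valid.
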(event OnComponentBeginOverlap(StaticMeshComponent)
  (params (OtherActor :type Actor%20Object%20Reference) (OtherComp :type Primitive%20Component%20Object%20Reference) (OtherBodyIndex :type Integer) (bFromSweep :type Boolean) (SweepResult :type Hit%20Result%20Structure%20%28by%20ref%29))
  (bind _otherportail (Variables|Default|GetOtherPortail))
  (if (Variables|Default|Getenabled)
    (bind _output_get (Variables|Default|SetSelectedPortail (Utilities|Array|Get(acopy) _otherportail (Math|Random|RandomIntegerinRange 0 (- (Utilities|Array|Length _otherportail) 1)))))
    (Variables|portail_C|Setenabled _output_get false)
    (Utilities|FlowControl|Delay (Utilities|Time|GetWorldDeltaSeconds))
    (Utilities|IsValid OtherActor
      (:Is%20Valid
        (Transformation|SetActorLocation OtherActor (Math|Vector|MakeVector (.x (Transformation|GetActorLocation (Variables|Default|GetSelectedPortail))) (.y (Transformation|GetActorLocation (Variables|Default|GetSelectedPortail))) (.z (Transformation|GetActorLocation OtherActor))) false true)
        (Variables|portail_C|Setenabled (Variables|Default|GetSelectedPortail) true)))))

(event EventBeginPlay)

(event EventActorBeginOverlap
  (params (OtherActor :type Actor%20Object%20Reference)))

(event EventTick
  (params (DeltaSeconds :type Float%20%28single-precision%29)))

(fn ConstructionScript)